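; BP_Bear is a bear monster that takes damage, flashes when hit and dissolves on death.
; Overlap with a "PlayerWeapon"-tagged actor plays a timeline-driven material hit effect, while AnyDamage separately forwards damage to BPHPController.
; The controller's death event switches the state enum, disables capsule collision and, after a delay, runs a dissolve timeline that destroys the actor when finished.
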(event `self.ReceiveActorBeginOverlap`
  (params (OtherActor :type "Actor Object Reference"))
  ;[0.06714 0.1268 0.15 0.5] Hit Effect 표현
  (if (`self.ActorHasTag` OtherActor "PlayerWeapon")
    (bind (_direction _hitvalue) (`Timeline|HitEffect` :!via `PlayFromStart`)
      (:`Update`
        (`MeshComponent.SetScalarParameterValueOnMaterials` (`self.Mesh`) "HitValue" _hitvalue)))))

(event `self.ReceiveAnyDamage`
  (params (Damage :type "Float (single-precision)") (DamageType :type "DamageType Object Reference") (InstigatedBy :type "Controller Object Reference") (DamageCauser :type "Actor Object Reference"))
  (`/Game/Blueprints/Components/BP_HPController.ReceiveDamage` (`self.BP_HPController`) Damage))

(event `self.ReceiveBeginPlay`
  ;[0.006293 0.15 0 0.5] 사망 이벤트 바인딩
  (add `/Game/Blueprints/Components/BP_HPController.OnDeadEvent` (`self.BP_HPController`) (delegate `ReceiveOnDead`)))

(event `ReceiveOnDead`
  (bind _mesh (`self.Mesh`))
  ;[0.006293 0.15 0 0.5] 사망 이벤트 바인딩
  (set `self.State_BP` "NewEnumerator3")
  (`PrimitiveComponent.SetCollisionEnabled` (`self.CapsuleComponent`) "NoCollision")
  ;[0.4918 0 0.04158 0.5] 사망 이벤트 이펙트
  (`KismetSystemLibrary.Delay` 2.0)
  (bind (_direction _dissolve _hitvalue) (`Timeline|DeathEffect` :!via `PlayFromStart`)
    (:`Update`
      (`MeshComponent.SetScalarParameterValueOnMaterials` _mesh "Dissolve" _dissolve)
      (`MeshComponent.SetScalarParameterValueOnMaterials` _mesh "Hitvalue" _hitvalue))
    (:`Finished`
      (`self.K2_DestroyActor`))))

(fn `UserConstructionScript`)