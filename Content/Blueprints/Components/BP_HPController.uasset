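; BP_HPController is a health component that tracks a character's HP and broadcasts death and health-change events.
; BeginPlay fills HealthPower to MaxHealthPower.
; ReceiveDamage subtracts damage only while HP is above zero, clamps it at zero and fires OnDead at that point, so death triggers once.
; Every applied hit then fires OnHpChanged with current and max HP.
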(event `ReceiveDamage`
  (params (Damage :type "Float (double-precision)"))
  ;[0.15 0.1008 0.003036 0.5] 체력 감소 처리 - 사망 & 체력변경 이벤트 발행
  (if (> (`self.HealthPower`) 0.0)
    ;; 체력 - 데미지
    (bind _output_get (set `self.HealthPower` (- (`self.HealthPower`) Damage)))
    ;; 남은 체력 <= 0
    (if (<= _output_get 0.0)
      (set `self.HealthPower` 0.0)
      (`self.OnDeadEvent`)
      (`self.OnHpChanged` (`self.HealthPower`) (`self.MaxHealthPower`)) ; 체력 값 변경 이벤트 발행
      (else
        (`self.OnHpChanged` (`self.HealthPower`) (`self.MaxHealthPower`)) ; 체력 값 변경 이벤트 발행
      ))))

(event `self.ReceiveBeginPlay`
  ;[0.15 0 0.04463 0.5] 시작할 때 최대체력 설정
  (set `self.HealthPower` (`self.MaxHealthPower`)))